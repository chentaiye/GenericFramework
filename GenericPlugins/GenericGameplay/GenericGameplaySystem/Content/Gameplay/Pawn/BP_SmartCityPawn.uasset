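; BP_SmartCityPawn is a player pawn that moves, turns and zooms through Enhanced Input.
; The move, turn and zoom actions pass their values straight to AddLocation, AddRotation and AddZoom, which are defined outside this graph.
; CanTouchMove and CanTouchTurn split touch control by screen half, allowing movement when the first touch position is left of the viewport center and turning when right.
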(event Input|EnhancedActionEvents|EnhancedInputActionIA_Move
  (params (ActionValue :type Vector%202D%20Structure) (ElapsedSeconds :type Float%20%28double-precision%29) (TriggeredSeconds :type Float%20%28double-precision%29) (InputAction :type Input%20Action%20Object%20Reference :default "/GenericCoreFramework/Input/MovementActions/IA_Move.IA_Move"))
  (Class|PawnInputMovementInterface|AddLocation ActionValue))

(event Input|EnhancedActionEvents|EnhancedInputActionIA_Turn
  (params (ActionValue :type Vector%202D%20Structure) (ElapsedSeconds :type Float%20%28double-precision%29) (TriggeredSeconds :type Float%20%28double-precision%29) (InputAction :type Input%20Action%20Object%20Reference :default "/GenericCoreFramework/Input/MovementActions/IA_Turn.IA_Turn"))
  (Class|PawnInputMovementInterface|AddRotation ActionValue))

(event Input|EnhancedActionEvents|EnhancedInputActionIA_Zoom
  (params (ActionValue :type Float%20%28double-precision%29) (ElapsedSeconds :type Float%20%28double-precision%29) (TriggeredSeconds :type Float%20%28double-precision%29) (InputAction :type Input%20Action%20Object%20Reference :default "/GenericCoreFramework/Input/MovementActions/IA_Zoom.IA_Zoom"))
  (Class|PawnInputMovementInterface|AddZoom ActionValue))

(fn ConstructionScript)

(fn CanTouchMove
  (return (< (.X (Math|Vector2D|BreakVector2D (Variables|Default|GetFirstTouchMovementPosition))) (/ (.x (Viewport|GetViewportSize)) 2.0))))

(fn CanTouchTurn
  (return (> (.X (Math|Vector2D|BreakVector2D (Variables|Default|GetFirstTouchMovementPosition))) (/ (.x (Viewport|GetViewportSize)) 2.0))))